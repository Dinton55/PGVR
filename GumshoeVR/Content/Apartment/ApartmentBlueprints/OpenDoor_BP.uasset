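; OpenDoor_BP is a trigger-operated two-part sliding door for the Apartment level.
; Overlapping the Trigger component plays two timelines, DoorOpenUP and DoorOpenDown, which lerp Door1 and Door2 relative locations from their closed to open vectors.
; Ending the overlap reverses both timelines, and neither overlap event filters by actor.
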(event OnComponentBeginOverlap(Trigger)
  (params (OverlappedComponent :type Primitive%20Component%20Object%20Reference) (OtherActor :type Actor%20Object%20Reference) (OtherComp :type Primitive%20Component%20Object%20Reference) (OtherBodyIndex :type Integer) (bFromSweep :type Boolean) (SweepResult :type Hit%20Result%20Structure%20%28by%20ref%29))
  (Utilities|FlowControl|Sequence
    (:then_0
      (bind _dooropendown (Timeline|DoorOpenDown Play)
        (:Update
          (Transformation|SetRelativeLocation (Variables|Default|GetDoor2) (Math|Vector|Lerp(Vector) (Variables|DoorSetup|GetDoor2%20Closed) (Variables|DoorSetup|GetDoor2%20Open) _dooropendown) false false))))
    (:then_1
      (bind _dooropenup (Timeline|DoorOpenUP Play)
        (:Update
          (Transformation|SetRelativeLocation (Variables|Default|GetDoor1) (Math|Vector|Lerp(Vector) (Variables|DoorSetup|GetDoor1%20Closed) (Variables|DoorSetup|GetDoor1%20Open) _dooropenup) false false))))))

(event OnComponentEndOverlap(Trigger)
  (params (OverlappedComponent :type Primitive%20Component%20Object%20Reference) (OtherActor :type Actor%20Object%20Reference) (OtherComp :type Primitive%20Component%20Object%20Reference) (OtherBodyIndex :type Integer))
  (Utilities|FlowControl|Sequence
    (:then_0
      (bind _dooropendown (Timeline|DoorOpenDown Reverse)
        (:Update
          (Transformation|SetRelativeLocation (Variables|Default|GetDoor2) (Math|Vector|Lerp(Vector) (Variables|DoorSetup|GetDoor2%20Closed) (Variables|DoorSetup|GetDoor2%20Open) _dooropendown) false false))))
    (:then_1
      (bind _dooropenup (Timeline|DoorOpenUP Reverse)
        (:Update
          (Transformation|SetRelativeLocation (Variables|Default|GetDoor1) (Math|Vector|Lerp(Vector) (Variables|DoorSetup|GetDoor1%20Closed) (Variables|DoorSetup|GetDoor1%20Open) _dooropenup) false false))))))

(fn ConstructionScript)