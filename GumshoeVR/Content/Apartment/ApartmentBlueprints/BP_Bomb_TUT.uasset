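; BP_Bomb_TUT is a tutorial bomb actor whose red wire is cut with scissors, marked as the game's win condition.
; When a BP_Scissors actor overlaps the red wire trigger, the uncut wire is hidden and the cut wire is shown.
; A DoOnce then plays the light tutorial voice-over, followed after a delay by the leave tutorial voice-over.
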(event OnComponentBeginOverlap(RedWireTrigger)
  (params (OverlappedComponent :type Primitive%20Component%20Object%20Reference) (OtherActor :type Actor%20Object%20Reference) (OtherComp :type Primitive%20Component%20Object%20Reference) (OtherBodyIndex :type Integer) (bFromSweep :type Boolean) (SweepResult :type Hit%20Result%20Structure%20%28by%20ref%29))
  ;[1 1 1] Game WIN
  (bind _asbp_scissors (Utilities|Casting|CastToBP_Scissors OtherActor))
  (if (Utilities|IsValid _asbp_scissors)
    (Rendering|SetVisibility (Variables|Default|GetRedWireUncut) false false)
    (Rendering|SetVisibility (Variables|Default|GetRedWireCut) true false)
    (Utilities|FlowControl|DoOnce false
      (:Completed
        (Audio|PlaySound2D "/Game/Sounds/NewTutorialVoicelines/LightTUT_01_VO.LightTUT_01_VO")
        (Utilities|FlowControl|Delay 8.0)
        (Audio|PlaySound2D "/Game/Sounds/NewTutorialVoicelines/LeaveTUT_01_VO.LeaveTUT_01_VO")))))

(event EventBeginPlay)

(event Collision|EventActorBeginOverlap
  (params (OtherActor :type Actor%20Object%20Reference)))

(event EventTick
  (params (DeltaSeconds :type Float%20%28single-precision%29)))

(fn ConstructionScript)