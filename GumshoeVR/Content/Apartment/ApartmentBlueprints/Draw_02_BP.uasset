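; Apartment drawer actor that slides along world X with the VR player's right motion controller.
; BeginPlay stores the start location and a limit MaxDist along +X.
; While the pawn's IsGrabbing is true, Tick copies the controller's X, without checking what is grabbed.
; Once the drawer is beyond MaxDist from the start in either direction, Tick sets it to the +X limit instead.
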(event EventBeginPlay
  (Variables|Default|SetInitialPosition (Transformation|GetActorLocation))
  (Variables|Default|SetMaxPosition (Math|Vector|MakeVector (+ (.X (Math|Vector|BreakVector (Variables|Default|GetInitialPosition))) (Variables|Default|GetMaxDist)) (.Y (Math|Vector|BreakVector (Variables|Default|GetInitialPosition))) (.Z (Math|Vector|BreakVector (Variables|Default|GetInitialPosition))))))

(event Collision|EventActorBeginOverlap
  (params (OtherActor :type Actor%20Object%20Reference)))

(event EventInteractable
  (params (Bool :type Boolean)))

(event EventTick
  (params (DeltaSeconds :type Float%20%28single-precision%29))
  (bind _returnvalue (Transformation|GetActorLocation))
  (bind (_x _y _z) (Math|Vector|BreakVector _returnvalue))
  (bind _asvr_conroller (Utilities|Casting|CastToVR_Conroller (Game|Player|GetPlayerPawn 0)))
  (if (Variables|/Game/CrossScene/Blueprints/VR_Conroller.VR_Conroller_C|GetIsGrabbing _asvr_conroller)
    (if (<= (Math|Vector|VectorLengthSquared (- (Transformation|GetActorLocation) (Variables|Default|GetInitialPosition))) (* (Variables|Default|GetMaxDist) (Variables|Default|GetMaxDist)))
      (Transformation|SetActorLocation (Math|Vector|MakeVector (.X (Math|Vector|BreakVector (Transformation|GetWorldLocation (Variables|/Game/CrossScene/Blueprints/VR_Conroller.VR_Conroller_C|GetMC_Right _asvr_conroller)))) _y _z) false false)
      (else
        (Transformation|SetActorLocation (Variables|Default|GetMaxPosition) false false)))))

(fn ConstructionScript)