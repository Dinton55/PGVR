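; Apartment drawer actor that the player slides along world X with the right VR motion controller.
; Overlapping its box makes it grabbable; while VR_Conroller is grabbing, Tick copies the hand's X to the drawer.
; If the hand leaves the MaxDist radius around the start position, the drawer snaps to just short of full extension on +X, whatever the direction.
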(event OnComponentBeginOverlap(BoxOG)
  (params (OverlappedComponent :type Primitive%20Component%20Object%20Reference) (OtherActor :type Actor%20Object%20Reference) (OtherComp :type Primitive%20Component%20Object%20Reference) (OtherBodyIndex :type Integer) (bFromSweep :type Boolean) (SweepResult :type Hit%20Result%20Structure%20%28by%20ref%29))
  (Variables|Default|SetbCanBeGrabbed true)
  (bind _asvr_conroller (Utilities|Casting|CastToVR_Conroller (Game|Player|GetPlayerPawn 0)))
  (if (Variables|/Game/CrossScene/Blueprints/VR_Conroller.VR_Conroller_C|GetIsGrabbing _asvr_conroller)
    _))

(event OnComponentEndOverlap(BoxOG)
  (params (OverlappedComponent :type Primitive%20Component%20Object%20Reference) (OtherActor :type Actor%20Object%20Reference) (OtherComp :type Primitive%20Component%20Object%20Reference) (OtherBodyIndex :type Integer))
  (Variables|Default|SetbCanBeGrabbed false))

(event EventBeginPlay
  (Variables|Default|SetInitialPosition (Transformation|GetActorLocation))
  (Variables|Default|SetMaxPosition (Math|Vector|MakeVector (+ (.X (Math|Vector|BreakVector (Variables|Default|GetInitialPosition))) (- (Variables|Default|GetMaxDist) 1.0)) (.Y (Math|Vector|BreakVector (Variables|Default|GetInitialPosition))) (.Z (Math|Vector|BreakVector (Variables|Default|GetInitialPosition))))))

(event EventInteractable
  (params (Bool :type Boolean)))

(event EventTick
  (params (DeltaSeconds :type Float%20%28single-precision%29))
  (bind _returnvalue (Transformation|GetActorLocation))
  (bind (_x _y _z) (Math|Vector|BreakVector _returnvalue))
  (bind _asvr_conroller (Utilities|Casting|CastToVR_Conroller (Game|Player|GetPlayerPawn 0)))
  (if (Variables|Default|GetbCanBeGrabbed)
    (if (Variables|/Game/CrossScene/Blueprints/VR_Conroller.VR_Conroller_C|GetIsGrabbing _asvr_conroller)
      (if (< (Math|Vector|VectorLengthSquared (- (Transformation|GetWorldLocation (Variables|/Game/CrossScene/Blueprints/VR_Conroller.VR_Conroller_C|GetMC_Right _asvr_conroller)) (Variables|Default|GetInitialPosition))) (* (Variables|Default|GetMaxDist) (Variables|Default|GetMaxDist)))
        (Transformation|SetActorLocation (Math|Vector|MakeVector (.X (Math|Vector|BreakVector (Transformation|GetWorldLocation (Variables|/Game/CrossScene/Blueprints/VR_Conroller.VR_Conroller_C|GetMC_Right _asvr_conroller)))) _y _z) false false)
        (else
          (Transformation|SetActorLocation (Variables|Default|GetMaxPosition) false false))))))

(fn ConstructionScript)