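; Level exit in the interrogation room that loads the Apartment level.
; An overlap on Box1 checks component tags for "White Card", with the other component's first tag deciding the result, then destroys the Cube and opens the level after a short delay.
; The Interactable event opens the same level if LockBroken is true, but the only node setting that flag here is disconnected.
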(event OnComponentBeginOverlap(Box1)
  (params (OverlappedComponent :type Primitive%20Component%20Object%20Reference) (OtherActor :type Actor%20Object%20Reference) (OtherComp :type Primitive%20Component%20Object%20Reference) (OtherBodyIndex :type Integer) (bFromSweep :type Boolean) (SweepResult :type Hit%20Result%20Structure%20%28by%20ref%29))
  (Utilities|FlowControl|Sequence
    (:then_0
      (Variables|Default|SetCardPresent (Utilities|Enum|Equal(Enum) (Utilities|String|ToString(Name) (Utilities|Array|Get(acopy) (Variables|/Script/Engine.ActorComponent|GetComponentTags OverlappedComponent))) "White Card"))
      (Variables|Default|SetCardPresent (Utilities|Enum|Equal(Enum) (Utilities|String|ToString(Name) (Utilities|Array|Get(acopy) (Variables|/Script/Engine.ActorComponent|GetComponentTags OtherComp))) "White Card")))
    (:then_1
      (if (Variables|Default|GetCardPresent)
        (Components|DestroyComponent (Variables|Default|GetCube))
        (Utilities|FlowControl|Delay 1.0)
        (Game|OpenLevel(byName) "Apartment")))))

(event EventInteractable
  (params (Bool :type Boolean))
  (if (Variables|Default|GetLock%20Broken)
    (Game|OpenLevel(byName) "Apartment")))

(fn ConstructionScript)