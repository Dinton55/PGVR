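; Reverse timer Blueprint that counts down minutes, seconds and hundredths and shows the result on the Time text.
; Tick runs through a Delay of DeltaSeconds, with a DoOnce reset wired back, decrementing MilSeconds per pass rather than by measured time.
; Underflow borrows from Seconds, then Minutes, with no stop at zero.
; Helper graphs zero-pad each unit before it is combined and displayed.
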(event Custom|Correct%20time%20%28Stirng%29
  (Utilities|CorrectMilSecond
    (:Out
      (Utilities|CorrectSeconds
        (:Out
          (Utilities|CorrectMiinutes
            (:Out
              (CallFunction|SetTimeShown))))))))

(event Custom|Set%20Time%20shown
  (bind _output_get (Variables|Default|SetShownTime (Utilities|ConverttoTime (Variables|Default|GetMilSecondsString) (Variables|Default|GetSecondString) (Variables|Default|GetMinutesString))))
  (Rendering|Components|TextRender|SetText (Variables|Default|GetTime) _output_get))

(event EventTick
  (params (DeltaSeconds :type Float%20%28single-precision%29))
  (Utilities|FlowControl|Delay DeltaSeconds)
  (Variables|Default|SetMilSeconds (- (Variables|Default|GetMilSeconds) 1) :!label _label)
  (Utilities|FlowControl|Sequence
    (:then_0
      (Utilities|FlowControl|DoOnce false ; enters at Reset
        (:Completed
          (goto _label))))
    (:then_1
      (if (== (Variables|Default|GetMilSeconds) -1)
        (Variables|Default|SetMilSeconds 99)
        (Variables|Default|SetSeconds (- (Variables|Default|GetSeconds) 1))
        (if (== (Variables|Default|GetSeconds) -1)
          (Variables|Default|SetSeconds 59)
          (Variables|Default|SetMinutes (- (Variables|Default|GetMinutes) 1))))
      (CallFunction|CorrectTime(Stirng)))))

(fn ConstructionScript)