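; Interactable interrogation light switch that raises and lowers a table through a level sequence.
; BeginPlay creates the table sequence player and starts a separate rotation sequence.
; While input is allowed, each interaction flip-flops the table sequence between forward and reverse playback and rotates the switch mesh.
; The first raise also starts a one-time delay that toggles the hologram and sets the table light if still rising.
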(event EventInteractable
  (params (Bool :type Boolean))
  (bind _sequencer (Variables|Default|GetSequencer))
  (bind _sequencer_2 (Variables|Default|GetSequencer))
  (bind _switchmesh (Variables|Default|GetSwitchMesh))
  (if (Variables|Default|GetCanTakeInput)
    (Utilities|FlowControl|FlipFlop
      (:A
        (Variables|Default|SetTableRising true)
        (Components|Timeline|SetPlayRate _sequencer 1.0)
        (Sequencer|Player|Play _sequencer :!class /Script/MovieScene.MovieSceneSequencePlayer)
        (Transformation|SetRelativeRotation _switchmesh "0, 0,-50.000000" false false)
        (Utilities|FlowControl|DoOnce false
          (:Completed
            (Utilities|FlowControl|Delay 3.0)
            (if (Variables|Default|GetTableRising)
              (Rendering|ToggleVisibility (Variables|Default|GetHologram) false)
              (Variables|Default|SetLightOn 2.5)
              (CallFunction|SetTableLight)
              (if (Variables|Default|GetTableRising)
                (Rendering|ToggleVisibility (Variables|Default|GetHologram) false)
                (Variables|Default|SetLightOn 2.5)
                (CallFunction|SetTableLight))))))
      (:B
        (Variables|Default|SetTableRising false)
        (Components|Timeline|SetPlayRate _sequencer_2 -1.0)
        (Sequencer|Player|Play _sequencer_2 :!class /Script/MovieScene.MovieSceneSequencePlayer)
        (Transformation|SetRelativeRotation _switchmesh "0, 0,-1400.000000" false false)))))

(event EventBeginPlay
  (bind _returnvalue (Sequencer|Player|CreateLevelSequencePlayer "/Game/Interegation_Room/TableRaise_Sec.TableRaise_Sec"))
  (Variables|Default|SetSequencer _returnvalue)
  (bind _returnvalue_2 (Sequencer|Player|CreateLevelSequencePlayer "/Game/Interegation_Room/Rotation.Rotation"))
  (bind _output_get (Variables|Default|SetRotation _returnvalue_2))
  (Sequencer|Player|Play _output_get :!class /Script/MovieScene.MovieSceneSequencePlayer))

(fn ConstructionScript)