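; Blood actor that lights up a hidden blood mark on its Cube when the player uses the VR UV blacklight.
; BeginPlay caches the VR_Conroller pawn; on a UVLight press, an active blacklight and a hit component tagged Dcl_01 set the material's BloodCol to orange-red.
; Tick resets BloodCol to black every frame, and both paths call CreateDynamicMaterialInstance each time rather than caching one.
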(event EventBeginPlay
  (bind _asvr_conroller (Utilities|Casting|CastToVR_Conroller (Game|Player|GetPlayerPawn 0)))
  (bind _output_get (Variables|Default|SetPlayer _asvr_conroller)))

(event Collision|EventActorBeginOverlap
  (params (OtherActor :type Actor%20Object%20Reference)))

(event EventTick
  (params (DeltaSeconds :type Float%20%28single-precision%29))
  (bind _cube (Variables|Default|GetCube))
  (bind _returnvalue (Rendering|Material|CreateDynamicMaterialInstance _cube 0 (Rendering|Material|GetMaterial _cube 0) :!class /Script/Engine.PrimitiveComponent))
  (Rendering|Material|SetVectorParameterValue _returnvalue "BloodCol" "(R=0.000000,G=0.000000,B=0.000000,A=1.000000)" :!class /Script/Engine.MaterialInstanceDynamic))

(event Input|ActionEvents|InputActionUVLight
  (params (Key :type Key%20Structure))
  (bind _cube (Variables|Default|GetCube))
  (:Pressed
    (if (Variables|/Game/CrossScene/Blueprints/VR_Conroller.VR_Conroller_C|GetBlacklighton (stale EventBeginPlay _output_get))
      (if (Utilities|Enum|Equal(Enum) "Dcl_01" (Utilities|String|ToString(Name) (Utilities|Array|Get(acopy) (Variables|/Script/Engine.ActorComponent|GetComponentTags (Variables|/Game/CrossScene/Blueprints/VR_Conroller.VR_Conroller_C|GetHit%20Component (stale EventBeginPlay _output_get))))))
        (bind _returnvalue (Rendering|Material|CreateDynamicMaterialInstance _cube 0 (Rendering|Material|GetMaterial _cube 0) :!class /Script/Engine.PrimitiveComponent))
        (Rendering|Material|SetVectorParameterValue _returnvalue "BloodCol" "(R=1.000000,G=0.180027,B=0.000000,A=1.000000)" :!class /Script/Engine.MaterialInstanceDynamic)))))

(fn ConstructionScript)