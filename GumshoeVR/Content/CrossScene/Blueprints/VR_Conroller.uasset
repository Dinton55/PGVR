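; VR player pawn with two-handed grabbing, snap turning, teleporting and widget interaction.
; Sphere traces attach physics objects to either hand, scanning shows their component tag, and grabbing messages overlapped interactables.
; Holding teleport traces for flat surfaces; releasing moves the pawn there at zero height.
; Flashlight and UV light work while held, with Tick feeding the UV light's position and direction into BloodSplat dynamic materials to render blacklight decals.
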(event OnComponentEndOverlap(InteractableCollision)
  (params (OverlappedComponent :type Primitive%20Component%20Object%20Reference) (OtherActor :type Actor%20Object%20Reference) (OtherComp :type Primitive%20Component%20Object%20Reference) (OtherBodyIndex :type Integer))
  ;[1 1 1] Dosen't do anything
  (Variables|Default|SetOverlappedComponent OverlappedComponent)
  (Variables|Default|SetOverlapped%20actor OtherActor)
  (Variables|Default|SetIsOverlappingInteractable false))

(event OnComponentEndOverlap(HandInteractiveCollisionRIGHT)
  (params (OverlappedComponent :type Primitive%20Component%20Object%20Reference) (OtherActor :type Actor%20Object%20Reference) (OtherComp :type Primitive%20Component%20Object%20Reference) (OtherBodyIndex :type Integer))
  ;[1 1 1] Dosen't do anything
  (Variables|Default|SetOverlappedComponent OverlappedComponent)
  (Variables|Default|SetOverlapped%20actor OtherActor)
  (Variables|Default|SetIsOverlappingInteractableRight false))

(event OnComponentBeginOverlap(InteractableCollision)
  (params (OverlappedComponent :type Primitive%20Component%20Object%20Reference) (OtherActor :type Actor%20Object%20Reference) (OtherComp :type Primitive%20Component%20Object%20Reference) (OtherBodyIndex :type Integer) (bFromSweep :type Boolean) (SweepResult :type Hit%20Result%20Structure%20%28by%20ref%29))
  ;[1 1 1] Dosen't do anything
  (Variables|Default|SetOverlappedComponent OverlappedComponent)
  (Variables|Default|SetOverlapped%20actor OtherActor)
  (Variables|Default|SetIsOverlappingInteractable true))

(event OnComponentBeginOverlap(HandInteractiveCollisionRIGHT)
  (params (OverlappedComponent :type Primitive%20Component%20Object%20Reference) (OtherActor :type Actor%20Object%20Reference) (OtherComp :type Primitive%20Component%20Object%20Reference) (OtherBodyIndex :type Integer) (bFromSweep :type Boolean) (SweepResult :type Hit%20Result%20Structure%20%28by%20ref%29))
  ;[1 1 1] Dosen't do anything
  (Variables|Default|SetOverlappedComponent OverlappedComponent)
  (Variables|Default|SetOverlapped%20actor OtherActor)
  (Variables|Default|SetIsOverlappingInteractableRight true))

(event Custom|PickupObject
  (bind _pickupleft (Variables|Default|GetPickupLeft))
  (bind _returnvalue (Transformation|GetWorldLocation _pickupleft))
  ;[1 1 1] Pickup Left
  (bind _outhit (Collision|SphereTraceForObjects _returnvalue _returnvalue 12.0 (Utilities|Array|MakeArray "ObjectTypeQuery4") false 0 "ForDuration"))
  (if true
    (Variables|Default|SetHit%20Component (.HitComponent (Collision|BreakHitResult _outhit)))
    (if (Physics|IsSimulatingPhysics (Variables|Default|GetHit%20Component) "None")
      (Variables|Default|SetIsHoldingObjectLeft true)
      (bind _output_get (Variables|Default|SetPickedUpActor (.HitActor (Collision|BreakHitResult _outhit))))
      (Physics|SetSimulatePhysics (Variables|Default|GetHit%20Component) false)
      (Transformation|AttachComponentToComponent _output_get (Variables|Default|GetHeldObjectLocationLeft) "None" "SnapToTarget" "SnapToTarget" "KeepWorld" true)
      (bind _output_get_2 (Variables|Default|SetDisplay%20Text%20Left (Utilities|Text|ToText(String) (Utilities|String|ToString(Name) (Utilities|Array|Get(acopy) (Variables|/Script/Engine.ActorComponent|GetComponentTags (.HitComponent (Collision|BreakHitResult _outhit)))))))))))

(event Custom|Dropbject
  ;[1 1 1] Drop Left
  (Utilities|IsValid (Variables|Default|GetPickedUpActor)
    (:Is%20Valid
      (Transformation|DetachFromActor (Variables|Default|GetPickedUpActor) "KeepWorld" "KeepWorld" "KeepWorld")
      (Utilities|IsValid (Variables|Default|GetHit%20Component)
        (:Is%20Valid
          (Physics|SetSimulatePhysics (Variables|Default|GetHit%20Component) true)
          (Variables|Default|SetIsHoldingObjectLeft false)
          (Variables|Default|SetHit%20Component 0)
          (Variables|Default|SetPickedUpActor 0)
          (bind _output_get (Variables|Default|SetDisplay%20Text%20Left (Variables|Default|GetClearText)))
          (Rendering|Components|TextRender|SetText (Variables|Default|GetTextRenderLeft) _output_get))))))

(event Custom|PickupObjectRight
  (bind _pickup_right (Variables|Default|GetPickup%20Right))
  (bind _returnvalue (Transformation|GetWorldLocation _pickup_right))
  ;[1 1 1] Pickup Right
  (bind _outhit (Collision|SphereTraceForObjects _returnvalue _returnvalue 12.0 (Utilities|Array|MakeArray "ObjectTypeQuery4") false 0 "ForDuration"))
  (if true
    (Variables|Default|SetHitComponentRight (.HitComponent (Collision|BreakHitResult _outhit)))
    (if (Physics|IsSimulatingPhysics (Variables|Default|GetHitComponentRight) "None")
      (Variables|Default|SetIsHoldingObjectRight? true)
      (bind _output_get (Variables|Default|SetPickedUpActorRight (.HitActor (Collision|BreakHitResult _outhit))))
      (Physics|SetSimulatePhysics (Variables|Default|GetHitComponentRight) false)
      (Transformation|AttachComponentToComponent _output_get (Variables|Default|GetHeldObjectLocationRight) "None" "SnapToTarget" "SnapToTarget" "KeepWorld" true))))

(event Custom|DropObjectRight
  ;[1 1 1] Drop Right
  (Utilities|IsValid (Variables|Default|GetPickedUpActorRight)
    (:Is%20Valid
      (Transformation|DetachFromActor (Variables|Default|GetPickedUpActorRight) "KeepWorld" "KeepWorld" "KeepWorld")
      (Utilities|IsValid (Variables|Default|GetHitComponentRight)
        (:Is%20Valid
          (Physics|SetSimulatePhysics (Variables|Default|GetHitComponentRight) true)
          (Variables|Default|SetIsHoldingObjectRight? false)
          (Variables|Default|SetHitComponentRight 0)
          (Variables|Default|SetPickedUpActorRight 0)
          (Rendering|Components|TextRender|SetText (Variables|Default|GetTextRenderRight) (Variables|Default|GetClearText)))))))

(event EventBeginPlay
  ;[1 1 1] Begin Play
  (Class|HeadMountedDisplayFunctionLibrary|SetTrackingOrigin "Floor")
  (Rendering|Components|Light|SetIntensity (Variables|Default|GetFlashlight) 0.0)
  (Rendering|Components|Light|SetIntensity (Variables|Default|GetUVLight) 0.0)
  (bind _returnvalue (UserInterface|CreateWidget "/Game/UserInterface/UI_PlayAreaWarning.UI_PlayAreaWarning_C"))
  (bind _output_get (Variables|Default|SetPlay%20Area%20UI _returnvalue))
  (UserInterface|Animation|PlayAnimation _output_get (Variables|/Game/UserInterface/UI_PlayAreaWarning.UI_PlayAreaWarning_C|GetAnimIn _output_get) 0.0 1 "Forward" 1.0))

(event EventPlayFadein
  (UserInterface|Animation|PlayAnimation (stale EventBeginPlay _output_get) (Variables|/Game/UserInterface/UI_PlayAreaWarning.UI_PlayAreaWarning_C|GetAnimIn (stale EventBeginPlay _output_get)) 0.0 1 "Forward" 1.0))

(event EventPlayFadeOut
  (UserInterface|Animation|PlayAnimation (stale EventBeginPlay _output_get) (Variables|/Game/UserInterface/UI_PlayAreaWarning.UI_PlayAreaWarning_C|GetAnimOut (stale EventBeginPlay _output_get)) 0.0 1 "Forward" 1.0))

(event EventTick
  (params (DeltaSeconds :type Float%20%28single-precision%29))
  (bind _raycastright (Variables|Default|GetRayCastRight))
  (bind _raycastleft (Variables|Default|GetRayCastLeft))
  (bind _uvlight (Variables|Default|GetUVLight))
  ;[1 1 1] Teleport
  (Utilities|FlowControl|Sequence
    (:then_0
      (if (Variables|Default|GetRightTeleportPressed?)
        (CallFunction|Teleport (Transformation|GetWorldLocation _raycastright) (Math|Vector|GetForwardVector _raycastright))))
    (:then_1
      (if (Variables|Default|GetLeftTeleportPressed?)
        (CallFunction|Teleport (Transformation|GetWorldLocation _raycastleft) (Math|Vector|GetForwardVector _raycastleft))))
    (:then_2
      (if (Variables|Default|GetBlacklighton)
        ;[1 1 1] Start Rendering light
        (bind _outactors (Actor|GetAllActorsOfClass "/Game/UVLight/BloodSplat.BloodSplat_C"))
        (for _array_element _outactors
          (Rendering|Material|SetVectorParameterValue (Variables|/Game/UVLight/BloodSplat.BloodSplat_C|GetMID _array_element) "BlackLightPos" (Math|Conversions|ToLinearColor(Vector) (Transformation|GetWorldLocation _uvlight)) :!class /Script/Engine.MaterialInstanceDynamic)
          (Rendering|Material|SetVectorParameterValue (Variables|/Game/UVLight/BloodSplat.BloodSplat_C|GetMID _array_element) "BlackLightDir" (Math|Conversions|ToLinearColor(Vector) (Math|Vector|GetForwardVector _uvlight)) :!class /Script/Engine.MaterialInstanceDynamic)
          (Rendering|Material|SetScalarParameterValue (Variables|/Game/UVLight/BloodSplat.BloodSplat_C|GetMID _array_element) "LightAngle" (Variables|Default|GetLightAngle) :!class /Script/Engine.MaterialInstanceDynamic)
          (Rendering|Material|SetScalarParameterValue (Variables|/Game/UVLight/BloodSplat.BloodSplat_C|GetMID _array_element) "LightFallOff" (Variables|Default|GetFallOff) :!class /Script/Engine.MaterialInstanceDynamic)
          (Rendering|Material|SetScalarParameterValue (Variables|/Game/UVLight/BloodSplat.BloodSplat_C|GetMID _array_element) "LightOn" 1.0 :!class /Script/Engine.MaterialInstanceDynamic))
        (else
          ;[1 1 1] Stop Rendering Blacklight Decals
          (bind _outactors_2 (Actor|GetAllActorsOfClass "/Game/UVLight/BloodSplat.BloodSplat_C"))
          (for _array_element_2 _outactors_2
            (Rendering|Material|SetScalarParameterValue (Variables|/Game/UVLight/BloodSplat.BloodSplat_C|GetMID _array_element_2) "LightOn" 0.0 :!class /Script/Engine.MaterialInstanceDynamic)))))))

(event Input|ActionEvents|InputActionGrabRight
  (params (Key :type Key%20Structure))
  ;[1 1 1] Grab/interact Right
  (:Pressed
    (if (not (Variables|Default|GetIsHoldingObjectRight?))
      (CallFunction|PickupObjectRight)
      (if (Variables|Default|GetIsOverlappingInteractableRight)
        (Class|PlayerInteract|Interactable(Message) (Variables|Default|GetOverlapped%20actor) true))))
  (:Released
    (CallFunction|DropObjectRight)))

(event Input|ActionEvents|InputActionUVLight
  (params (Key :type Key%20Structure))
  ;[1 1 1] FlashLight
  (:Pressed
    (Utilities|FlowControl|DoOnce false :!label _label
      (:Completed
        (Rendering|Components|Light|SetIntensity (Variables|Default|GetUVLight) 5e+03)
        (Variables|Default|SetBlacklighton true)
        (goto _label_2 Reset))))
  (:Released
    (Utilities|FlowControl|DoOnce false :!label _label_2
      (:Completed
        (Rendering|Components|Light|SetIntensity (Variables|Default|GetUVLight) 0.0)
        (Variables|Default|SetBlacklighton false)
        (goto _label Reset)))))

(event Input|ActionEvents|InputActionTeleportLeft
  (params (Key :type Key%20Structure))
  (bind _rightteleportpressed_ (Variables|Default|GetRightTeleportPressed?))
  ;[1 1 1] Teleport
  (:Pressed
    (if (not _rightteleportpressed_)
      (Variables|Default|SetLeftTeleportPressed? true)))
  (:Released
    (if (not _rightteleportpressed_)
      (Variables|Default|SetLeftTeleportPressed? false)
      (if (Variables|Default|GetCanTeleport?)
        (Utilities|FlowControl|Delay 0.3)
        (CallFunction|TeleporttoLocation (Variables|Default|GetTeleportLocation))))))

(event Input|ActionEvents|InputActionTeleportRight
  (params (Key :type Key%20Structure))
  (bind _leftteleportpressed_ (Variables|Default|GetLeftTeleportPressed?))
  ;[1 1 1] Teleport
  (:Pressed
    (if (not _leftteleportpressed_)
      (Variables|Default|SetRightTeleportPressed? true)))
  (:Released
    (if (not _leftteleportpressed_)
      (Variables|Default|SetRightTeleportPressed? false)
      (if (Variables|Default|GetCanTeleport?)
        (Utilities|FlowControl|Delay 0.3)
        (CallFunction|TeleporttoLocation (Variables|Default|GetTeleportLocation))))))

(event Input|ActionEvents|InputActionRotateRight
  (params (Key :type Key%20Structure))
  (bind _vrcameraroot (Variables|Default|GetVRCameraRoot))
  (bind _returnvalue (Transformation|GetWorldRotation _vrcameraroot))
  (bind (_roll _pitch _yaw) (Math|Rotator|BreakRotator _returnvalue))
  ;[1 1 1] Rotate
  (:Pressed
    (Transformation|SetWorldRotation _vrcameraroot (Math|Rotator|MakeRotator _roll _pitch (+ _yaw 3e+01)) false false)))

(event Input|ActionEvents|InputActionRotateLeft
  (params (Key :type Key%20Structure))
  (bind _vrcameraroot (Variables|Default|GetVRCameraRoot))
  (bind _returnvalue (Transformation|GetWorldRotation _vrcameraroot))
  (bind (_roll _pitch _yaw) (Math|Rotator|BreakRotator _returnvalue))
  ;[1 1 1] Rotate
  (:Pressed
    (Transformation|SetWorldRotation _vrcameraroot (Math|Rotator|MakeRotator _roll _pitch (- _yaw 3e+01)) false false)))

(event Input|ActionEvents|InputActionFlashLight
  (params (Key :type Key%20Structure))
  ;[1 1 1] FlashLight
  (:Pressed
    (Utilities|FlowControl|DoOnce false :!label _label
      (:Completed
        (Rendering|Components|Light|SetIntensity (Variables|Default|GetFlashlight) 9e+03)
        (goto _label_2 Reset))))
  (:Released
    (Utilities|FlowControl|DoOnce false :!label _label_2
      (:Completed
        (Rendering|Components|Light|SetIntensity (Variables|Default|GetFlashlight) 0.0)
        (goto _label Reset)))))

(event Input|ActionEvents|InputActionScanRight
  (params (Key :type Key%20Structure))
  ;[1 1 1] Pickup Right
  (:Pressed
    (if (Variables|Default|GetIsHoldingObjectRight?)
      (Rendering|Components|TextRender|SetText (Variables|Default|GetTextRenderRight) (Utilities|Text|ToText(String) (Utilities|String|ToString(Name) (Utilities|Array|Get(acopy) (Variables|/Script/Engine.ActorComponent|GetComponentTags (.HitComponent (Collision|BreakHitResult (stale Custom|PickupObjectRight _outhit)))))))))))

(event Input|ActionEvents|InputActionScanLeft
  (params (Key :type Key%20Structure))
  ;[1 1 1] Pickup Left
  (:Pressed
    (if (Variables|Default|GetIsHoldingObjectLeft)
      (Rendering|Components|TextRender|SetText (Variables|Default|GetTextRenderLeft) (stale Custom|PickupObject _output_get_2)))))

(event Input|ActionEvents|InputActionGrabLeft
  (params (Key :type Key%20Structure))
  ;[1 1 1] Grab/Interact Left
  (:Pressed
    (if (not (Variables|Default|GetIsHoldingObjectLeft))
      (CallFunction|PickupObject)
      (if (Variables|Default|GetIsOverlappingInteractable)
        (Class|PlayerInteract|Interactable(Message) (Variables|Default|GetOverlapped%20actor) true))))
  (:Released
    (CallFunction|Dropbject)))

(event Input|KeyboardEvents|MotionControllerRightGrip1
  (params (Key :type Key%20Structure))
  (bind _pointlight (Variables|Default|GetPointLight))
  (bind _widgetinteraction (Variables|Default|GetWidgetInteraction))
  ;[1 1 1] Widget interact
  (:Pressed
    (Class|WidgetInteractionComponent|PressPointerKey _widgetinteraction "LeftMouseButton")
    (Rendering|Components|Light|SetLightColor _pointlight "(R=0.093206,G=0.000000,B=1.000000,A=1.000000)" true))
  (:Released
    (Class|WidgetInteractionComponent|ReleasePointerKey _widgetinteraction "LeftMouseButton")
    (Rendering|Components|Light|SetLightColor _pointlight "(R=1.000000,G=0.919592,B=0.000000,A=1.000000)" true)))

(fn ConstructionScript)

(fn Teleport
  (params (Position :type Vector) (ForwardVector :type Vector))
  (bind _outhit (Collision|LineTraceByChannel Position (+ Position (* ForwardVector 1e+03)) "TraceTypeQuery1" false 0 "ForOneFrame"))
  (bind _output_get (Variables|Default|SetCanTeleport? (> (Math|Vector|DotProduct (.Normal (Collision|BreakHitResult _outhit)) "0, 0,1.000000") 0.9)))
  (if _output_get
    (bind _output_get_2 (Variables|Default|SetTeleportLocation (.Location (Collision|BreakHitResult _outhit))))
    (Class|KismetSystemLibrary|DrawDebugCylinder _output_get_2 (+ _output_get_2 (* (.Normal (Collision|BreakHitResult _outhit)) 2e+01)) 2e+01 12 "(R=1.000000,G=1.000000,B=1.000000,A=1.000000)" 0.0 0.0)))

(fn TeleporttoLocation
  (params (Location :type Vector))
  (bind (_x _y) (Math|Vector|BreakVector Location))
  (Transformation|SetActorLocation (Math|Vector|MakeVector _x _y 0.0) false true))