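; World-placed clock actor that shows a running HH:MM:SS time and an FPS counter, turning on the horizontal plane to face the player.
; Tick uses a one-second Delay with DoOnce to count seconds, rolling them into minutes and hours.
; Correct macros zero-pad each unit before the formatted time is set on TimeShown and debug-printed.
; A shorter Delay refreshes the FPS text from the inverse of DeltaSeconds.
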(event Custom|Correct%20Time
  ;[1 1 1] Set time
  (Utilities|CorrectSeconds
    (:Out
      (Utilities|CorrectMinutes
        (:Out
          (Utilities|CorrectHours
            (:Out
              (CallFunction|SetCurrentTime))))))))

(event Custom|Set%20Current%20Time
  ;[1 1 1] Set time
  (bind _output_get (Variables|Default|SetTime (Utilities|ConverttoTime (Variables|Default|GetSeconds%20String) (Variables|Default|GetMinutes%20String) (Variables|Default|GetHours%20String))))
  (Rendering|Components|TextRender|SetText (Variables|Default|GetTimeShown) _output_get))

(event EventTick
  (params (DeltaSeconds :type Float%20%28single-precision%29))
  ;[1 1 1] Set time
  (Utilities|FlowControl|Sequence
    (:then_0
      (Utilities|FlowControl|Delay 1.0)
      (Utilities|FlowControl|DoOnce false :!label _label
        (:Completed
          (Variables|Default|SetSeconds_Int (+ (Variables|Default|GetSeconds_Int) 1))
          (Utilities|FlowControl|Sequence
            (:then_0
              (goto _label Reset))
            (:then_1
              (if (== (Variables|Default|GetSeconds_Int) 60)
                (Variables|Default|SetSeconds_Int 0)
                (Variables|Default|SetMinutes_Int (+ (Variables|Default|GetMinutes_Int) 1))
                (if (== (Variables|Default|GetMinutes_Int) 60)
                  (Variables|Default|SetMinutes_Int 0)
                  (Variables|Default|SetHours_Int (+ (Variables|Default|GetHours_Int) 1))))
              (CallFunction|CorrectTime)
              (Development|PrintString (Utilities|String|ToString(Text) (Variables|Default|GetTime))))))))
    (:then_1
      ;[1 1 1] Face Player
      (Transformation|SetActorRotation (Math|Conversions|RotationFromXVector (Math|Vector|RotateVector (Math|Vector|Normalize (* (- (Transformation|GetActorLocation (Game|Player|GetPlayerPawn 0)) (Transformation|GetActorLocation)) "1.000000,1.000000, 0")) "0, 0, 0"))))
    (:then_2
      (Utilities|FlowControl|Delay 0.1)
      (bind _output_get (Variables|Default|SetFPSText (Utilities|Text|ToText(Integer) (Math|Float|Round (/ 1.0 DeltaSeconds)))))
      (Rendering|Components|TextRender|SetText (Variables|Default|GetFPS%20Counter) _output_get))))

(fn ConstructionScript)